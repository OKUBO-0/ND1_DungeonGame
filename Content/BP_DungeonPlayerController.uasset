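; BP_DungeonPlayerController is the player controller that turns Enhanced Input into pawn movement and camera orbit.
; BeginPlay registers the IMC_Game mapping context.
; IA_Move combines the camera manager's flattened forward vector and its right vector, then normalizes the sum so diagonal movement stays even.
; IA_CameraController feeds yaw input to the controlled pawn, negated when CameraYawInverse is set.
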(event `self.ReceiveBeginPlay`
  ; 2-1: Register the Enhanced Input mapping context
  (`EnhancedInputSubsystemInterface.AddMappingContext` (pcsubsystem `EnhancedInputLocalPlayerSubsystem` self) "/Game/IMC_Game.IMC_Game" 0 (struct)))

(event `EnhancedInput|/Game/IA_Move`
  (params (ActionValue :type "Vector2D Structure") (ElapsedSeconds :type "Float (double-precision)") (TriggeredSeconds :type "Float (double-precision)") (InputAction :type "InputAction Object Reference" :default "/Game/IA_Move.IA_Move"))
  (bind _returnvalue (`GameplayStatics.GetPlayerCameraManager` 0))
  (bind (_x _y) (`KismetMathLibrary.BreakVector2D` ActionValue))
  ; 2-1: Camera-relative movement on the XY plane; normalize diagonal input
  (:`Triggered`
    (`Pawn.AddMovementInput` (`self.K2_GetPawn`) (`KismetMathLibrary.Normal` (+ (* (`KismetMathLibrary.Vector_Normal2D` (`self.GetActorForwardVector` _returnvalue)) _y) (* (`self.GetActorRightVector` _returnvalue) _x))) 1.0 false)))

(event `EnhancedInput|/Game/IA_CameraController`
  (params (ActionValue :type "Float (double-precision)") (ElapsedSeconds :type "Float (double-precision)") (TriggeredSeconds :type "Float (double-precision)") (InputAction :type "InputAction Object Reference" :default "/Game/IA_CameraController.IA_CameraController"))
  ; 2-1: Arrow-key camera orbit with optional CameraYawInverse
  (:`Triggered`
    (`Pawn.AddControllerYawInput` (`self.K2_GetPawn`) (`KismetMathLibrary.SelectFloat` (* ActionValue -1.0) ActionValue (`self.CameraYawInverse`)))))

(fn `UserConstructionScript`)